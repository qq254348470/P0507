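; Game instance Blueprint that owns the game's BP_Save save object for a single save slot.
; On Init it loads the existing slot or creates a new save object, caches it and writes it back to the slot.
; LoadSlotCF returns the cached save, creating and saving one if it is invalid, and SaveSlotCF writes it to the slot.
; An unconnected debug chain prints the first StructSave entry.
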(event EventInit
  (bind _returnvalue (SaveGame|DoesSaveGameExist (Variables|Default|GetSaveSlot)))
  (if _returnvalue
    (bind _returnvalue_2 (SaveGame|LoadGamefromSlot (Variables|Default|GetSaveSlot)))
    (bind _asbp_save (Utilities|Casting|CastToBP_Save _returnvalue_2))
    (Variables|Default|SetBP_Save _asbp_save)
    (SaveGame|SaveGametoSlot (Variables|Default|GetBP_Save) (Variables|Default|GetSaveSlot))
    (else
      (bind _returnvalue_3 (SaveGame|CreateSaveGameObject "/Game/Game/BP_Save.BP_Save_C"))
      (Variables|Default|SetBP_Save _returnvalue_3)
      (SaveGame|SaveGametoSlot (Variables|Default|GetBP_Save) (Variables|Default|GetSaveSlot))
      (Development|PrintString "Hello++Create" true true "(R=1.000000,G=0.039974,B=0.000000,A=1.000000)" 5.0))))

(fn LoadSlotCF
  (Utilities|IsValid (Variables|Default|GetBP_Save)
    (:Is%20Valid
      _)
    (:Is%20Not%20Valid
      (bind _returnvalue (SaveGame|CreateSaveGameObject "/Game/Game/BP_Save.BP_Save_C"))
      (Variables|Default|SetBP_Save _returnvalue)
      (SaveGame|SaveGametoSlot (Variables|Default|GetBP_Save) (Variables|Default|GetSaveSlot))))
  (return (Variables|Default|GetBP_Save)))

(fn SaveSlotCF
  (SaveGame|SaveGametoSlot (Variables|Default|GetBP_Save) (Variables|Default|GetSaveSlot)))