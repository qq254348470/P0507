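; BP_Player is a player Blueprint that links the main and server UMG screens to saved "CS" entries and parameter-driven audio playback.
; BeginPlay shows the cursor and caches the server or main widget from BP_Controller by authority.
; CS_Send writes entries to the game instance's save object and lists them in the server widget.
; Play_CS clears audio integer parameters, enables the selected keys and plays, while RemoveMain_CS removes main widgets.
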(event Custom|CS_Send
  (params (Array :type Array%20of%20Struct%20Save%20Structures))
  (bind _asbp_instance (Utilities|Casting|CastToBP_Instance (Game|GetGameInstance)))
  (Variables|/Game/Game/BP_Save.BP_Save_C|SetStruct_Save (Variables|/Game/Game/BP_Instance.BP_Instance_C|GetBP_Save _asbp_instance) Array)
  (bind _foundwidgets (Widget|GetAllWidgetsOfClass "/Game/UI/Game/Server_UMG.Server_UMG_C" false))
  (Variables|Default|SetServerUMG (Utilities|Array|Get(acopy) _foundwidgets))
  (for _array_element Array
    (Default|AddCS (Variables|Default|GetServerUMG) "" _array_element)))

(event Custom|Play_CS
  (params (Index :type Array%20of%20Strings) (AllKey :type Array%20of%20Strings))
  (bind _audio (Variables|Default|GetAudio))
  (Effects|Components|ParticleSystem|SetIntParameter (Variables|Default|GetAudio) "00" 0)
  (CallFunction|ClearCS AllKey)
  (for _array_element Index
    (Effects|Components|ParticleSystem|SetIntParameter (Variables|Default|GetAudio) (Utilities|String|StringToName _array_element) 1)
    (Development|PrintString _array_element true true "(R=1.000000,G=0.000000,B=0.220988,A=1.000000)" 1e+01))
  (Effects|Components|ParticleSystem|SetIntParameter _audio "00" 1)
  (Audio|Components|Audio|Play _audio 0.0))

(event Custom|Clear_CS
  (params (AllKey :type Array%20of%20Strings))
  (for _array_element AllKey
    (Effects|Components|ParticleSystem|SetIntParameter (Variables|Default|GetAudio) (Utilities|String|StringToName _array_element) 0)))

(event Custom|13123
  (bind _foundwidgets (Widget|GetAllWidgetsOfClass "/Game/UI/Game/MainUMG.MainUMG_C" false))
  (Development|PrintString (Utilities|String|ToString(Integer) (Utilities|Array|Length _foundwidgets)) true true "(R=0.000000,G=0.660000,B=1.000000,A=1.000000)" 2e+01)
  (for _array_element _foundwidgets
    (Widget|RemovefromParent _array_element)))

(event Custom|RemoveMain_CS
  (CallFunction|13123))

(event Collision|EventActorBeginOverlap
  (params (OtherActor :type Actor%20Object%20Reference)))

(event EventBeginPlay
  (bind _returnvalue (Game|GetPlayerController 0))
  (bind _asbp_instance (Utilities|Casting|CastToBP_Instance (Game|GetGameInstance)))
  (Variables|Default|SetBP_Instance _asbp_instance)
  (Variables|/Script/Engine.PlayerController|SetbShowMouseCursor _returnvalue true)
  (bind _asbp_controller (Utilities|Casting|CastToBP_Controller _returnvalue))
  (Networking|SwitchHasAuthority
    (:Authority
      (Variables|Default|SetServerUMG (Variables|/Game/BP/BP_Controller.BP_Controller_C|GetServerUMG _asbp_controller)))
    (:Remote
      (Variables|Default|SetMainUMG (Variables|/Game/BP/BP_Controller.BP_Controller_C|GetMainUMG _asbp_controller)))))

(fn ConstructionScript)