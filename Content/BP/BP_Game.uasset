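; Game mode that acts as the server-side hub for a multiplayer session, tracking joined controllers and names and creating each player's UI on login.
; Rebuilds per-player info and total scores from every controller except the first to join.
; Relays UI sync, audio, click and drawing events by looping over controllers, with some relays skipping that first player, likely the host.
; Logout removes the player and calls QuitGame on that controller.
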(event Custom|SendCopy_CS
  (params (TargetKey :type String) (A :type Text) (B :type Text) (True :type Array%20of%20Booleans) (Score :type Integer))
  ;[1 1 1] Copy__0101
  (for (_array_element _array_index) (Variables|Default|GetPlayer)
    (bind _asbp_controller (Utilities|Casting|CastToBP_Controller _array_element))
    (if (>= _array_index 1)
      (Default|UpdateCopyCS _asbp_controller TargetKey A B True Score))))

(event Custom|GetAllPlayerMsg_CS
  (params (Name :type Text%20%28by%20ref%29))
  ;[1 1 1] 添加信息
  (Utilities|Array|Add (Variables|Default|GetName) Name))

(event Custom|GM_PlayAduio_CS
  (params (Index :type Integer))
  (for _array_element (Variables|Default|GetPlayer)
    (bind _asbp_controller (Utilities|Casting|CastToBP_Controller _array_element))
    (Default|ClientPlayAuidoCS _asbp_controller Index)))

(event Custom|QuitGM_CS
  (params (Controller :type BP%20Controller%20Object%20Reference%20%28by%20ref%29))
  (Utilities|Array|RemoveItem (Variables|Default|GetName) (Variables|/Game/BP/BP_Controller.BP_Controller_C|GetName Controller))
  (Utilities|Array|RemoveItem (Variables|Default|GetPlayer) Controller)
  (Game|QuitGame Controller "Quit" true))

(event Custom|OpenDraw_CS
  (params (Color :type Linear%20Color%20Structure%20%28by%20ref%29))
  (for _array_element (Variables|Default|GetPlayer)
    (bind _asbp_controller (Utilities|Casting|CastToBP_Controller _array_element))
    (Default|OpenDrawMenuCS _asbp_controller Color)))

(event Custom|GetOtherInfo_CS
  ;[1 1 1] 获取其他玩家信息
  (Utilities|Array|Clear (Variables|Default|GetGM))
  (for (_array_element _array_index) (Variables|Default|GetPlayer)
    (if (> _array_index 0)
      (bind _asbp_controller (Utilities|Casting|CastToBP_Controller _array_element))
      (Utilities|Array|Add (Variables|Default|GetGM) (Utilities|Struct|MakeStructGM (Variables|/Game/BP/BP_Controller.BP_Controller_C|GetName _asbp_controller) (Variables|/Game/BP/BP_Controller.BP_Controller_C|GetStruct_Save _asbp_controller)))))
  (Utilities|Array|Clear (Variables|Default|GetMainScore))
  (for _array_element_2 (Variables|Default|GetGM)
    (Variables|Default|SetScore 0)
    (for _array_element_3 (.Info (Utilities|Struct|BreakStructGM _array_element_2))
      (Variables|Default|SetScore (+ (.Score (Utilities|Struct|BreakStruct_Save _array_element_3)) (Variables|Default|GetScore))))
    (Utilities|Array|Add (Variables|Default|GetMainScore) (Variables|Default|GetScore))))

(event Custom|CopyPlayAudio_CS
  (params (Index :type Array%20of%20Strings) (AllKey :type Array%20of%20Strings))
  ;[1 1 1] 同步：播放声音
  (for _array_element (Variables|Default|GetPlayer)
    (bind _asbp_controller (Utilities|Casting|CastToBP_Controller _array_element))
    (bind _asbp_player (Utilities|Casting|CastToBP_Player (Pawn|GetControlledPawn _asbp_controller)))
    (Default|PlayCS _asbp_player Index AllKey)))

(event Custom|AllStartCopyUI_CS
  ;[1 1 1] 广播同步UI
  (for _array_element (Variables|Default|GetPlayer)
    (bind _asbp_controller (Utilities|Casting|CastToBP_Controller _array_element))
    (Default|MultCopyUICS _asbp_controller)))

(event Custom|CallAllCopuUI_CS
  (params (CopyState_E :type CopyState_E%20Enum :default "NewEnumerator2"))
  ;[1 1 1] 同步
  (for _array_element (Variables|Default|GetPlayer)
    (bind _asbp_controller (Utilities|Casting|CastToBP_Controller _array_element))
    (Variables|/Game/BP/BP_Controller.BP_Controller_C|SetCopyState_E _asbp_controller CopyState_E)))

(event Custom|CopyClickedInfo_CS
  (params (Key :type String) (Select :type Boolean) (Index :type Integer))
  ;[1 1 1] Copy__0202
  (for (_array_element _array_index) (Variables|Default|GetPlayer)
    (bind _asbp_controller (Utilities|Casting|CastToBP_Controller _array_element))
    (if (>= _array_index 1)
      (Default|Copy0202ClickedCS _asbp_controller Key Select Index))))

(event Custom|CopyClearInfo_CS
  ;[1 1 1] Copy__0202
  (for _array_element (Variables|Default|GetPlayer)
    (bind _asbp_controller (Utilities|Casting|CastToBP_Controller _array_element))
    (Default|CopyClearUICS _asbp_controller)))

(event Custom|StartDraw_CS
  (params (Draw :type Array%20of%20Struct%20Draw%20Structures))
  (for (_array_element _array_index) (Variables|Default|GetPlayer)
    (bind _asbp_controller (Utilities|Casting|CastToBP_Controller _array_element))
    (if (>= _array_index 1)
      (Default|StartDrawCS _asbp_controller Draw))))

(event Custom|GM_Clicked_CS
  (params (Index :type Integer%20%28by%20ref%29))
  (for _array_element (Variables|Default|GetPlayer)
    (bind _asbp_controller (Utilities|Casting|CastToBP_Controller _array_element))
    (Default|ClientClickedCS _asbp_controller Index)))

(event EventOnLogout
  (params (ExitingController :type Controller%20Object%20Reference))
  ;[1 1 1] 客户端退出
  (bind _asbp_controller (Utilities|Casting|CastToBP_Controller ExitingController))
  (CallFunction|QuitGMCS _asbp_controller))

(event EventPostLogin
  (params (NewPlayer :type Player%20Controller%20Object%20Reference))
  ;[1 1 1] 玩家登陆
  (Utilities|Array|Add (Variables|Default|GetPlayer) NewPlayer)
  (bind _asbp_controller (Utilities|Casting|CastToBP_Controller NewPlayer))
  (Default|CreateUICS _asbp_controller))

(fn ConstructionScript)