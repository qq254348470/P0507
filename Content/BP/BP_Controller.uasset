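; Player controller Blueprint that sets up role-specific UI and relays messages to the game mode.
; CreateUI_CS creates one Server_UMG widget on the server or one MainUMG widget otherwise, guarding against duplicates.
; SendMsg_CS passes a message and item to BP_Game's GetAllPlayerMsgCS.
; AddToUI_CS fills the server widget from parallel arrays of names and save structs, one AddCS call per entry.
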(event Custom|AddToUI_CS
  (params (NewParam :type Array%20of%20Struct%20Save%20Structures) (NewParam2 :type Array%20of%20Texts))
  (bind _serverumg (Variables|Default|GetServerUMG))
  (Utilities|IsValid _serverumg
    (:Is%20Valid
      (for (_array_element _array_index) NewParam
        (Default|AddCS _serverumg (Utilities|Array|Get(acopy) NewParam2 _array_index) _array_element)))))

(event Custom|CreateUI_CS
  (if (Networking|IsServer)
    (Utilities|IsValid (Variables|Default|GetServerUMG)
      (:Is%20Not%20Valid
        (bind _returnvalue (UserInterface|CreateWidget "/Game/UI/Game/Server_UMG.Server_UMG_C"))
        (bind _output_get (Variables|Default|SetServerUMG _returnvalue))
        (UserInterface|Viewport|AddtoViewport _output_get 0)))
    (else
      (Utilities|IsValid (Variables|Default|GetMainUMG)
        (:Is%20Not%20Valid
          (bind _returnvalue_2 (UserInterface|CreateWidget "/Game/UI/Game/MainUMG.MainUMG_C"))
          (bind _output_get_2 (Variables|Default|SetMainUMG _returnvalue_2))
          (UserInterface|Viewport|AddtoViewport _output_get_2 0))))))

(event Custom|SendMsg_CS
  (params (Msg :type Struct%20Save%20Structure) (NewItem :type Text%20%28by%20ref%29))
  (bind _asbp_game (Utilities|Casting|CastToBP_Game (Game|GetGameMode)))
  (Default|GetAllPlayerMsgCS _asbp_game Msg NewItem))

(fn ConstructionScript)