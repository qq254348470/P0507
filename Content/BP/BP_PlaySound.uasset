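; BP_PlaySound plays key-selected sound through an audio component and reports saved score data on screen.
; Play_CS clears all keys, sets an integer parameter named after each requested key to 1, toggles the "00" parameter around the update, then restarts the audio.
; CS_Send lazily creates a Server_UMG widget, then prints the first save entry's Score and adds it to that widget.
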(event Custom|CS_Send
  (params (Struct_Save :type Array%20of%20Struct%20Save%20Structures))
  (bind _output (Utilities|Array|Get(acopy) Struct_Save))
  (bind _score (Utilities|Struct|BreakStruct_Save _output))
  (bind _returnvalue (Utilities|String|ToString(Integer) _score))
  (Utilities|IsValid (Variables|Default|GetNewVar_2)
    (:Is%20Valid
      _)
    (:Is%20Not%20Valid
      (bind _returnvalue_2 (UserInterface|CreateWidget "/Game/UI/Game/Server_UMG.Server_UMG_C"))
      (bind _output_get (Variables|Default|SetNewVar_2 _returnvalue_2))
      (UserInterface|Viewport|AddtoViewport _output_get 0)))
  (Development|PrintString _returnvalue)
  (Default|AddCS (Variables|Default|GetNewVar_2) (Utilities|Text|ToText(String) _returnvalue)))

(event Custom|Play_CS
  (params (Index :type Array%20of%20Strings) (AllKey :type Array%20of%20Strings))
  (bind _audio (Variables|Default|GetAudio))
  (Effects|Components|ParticleSystem|SetIntParameter (Variables|Default|GetAudio) "00" 0)
  (CallFunction|ClearCS AllKey)
  (for _array_element Index
    (Effects|Components|ParticleSystem|SetIntParameter (Variables|Default|GetAudio) (Utilities|String|StringToName _array_element) 1)
    (Development|PrintString _array_element true true "(R=1.000000,G=0.000000,B=0.220988,A=1.000000)" 1e+01))
  (Effects|Components|ParticleSystem|SetIntParameter _audio "00" 1)
  (Audio|Components|Audio|Play _audio 0.0))

(event Custom|Clear_CS
  (params (AllKey :type Array%20of%20Strings))
  (for _array_element AllKey
    (Effects|Components|ParticleSystem|SetIntParameter (Variables|Default|GetAudio) (Utilities|String|StringToName _array_element) 0)))

(fn ConstructionScript)